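; Extractable tooth actor that can be rotated by a slider value and flags when it has been extracted.
; On BeginPlay it stores the tooth's starting height and mesh reference, clears selection and rolls a random WiggleHP, which this graph never decrements.
; While selected, UpdateSMRotation maps Rotation01 to a roll within MaxAngle either side of 90 degrees.
; When the mesh overlaps BoxCollision, it is destroyed and ExtractionDone is set.
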(event `self.ReceiveBeginPlay`
  (bind (_returnvalue_x _returnvalue_y _returnvalue_z) (`KismetMathLibrary.BreakVector` (`SceneComponent.K2_GetComponentLocation` (`self.StaticMesh`))))
  ; Extractable initialization
  (set `self.OriginalToothZ` _returnvalue_z)
  (set `self.IsThisExtractableSelected` false)
  (set `self.Ref_SM` (`self.StaticMesh`))
  (set `self.WiggleHP` (`KismetMathLibrary.RandomIntegerInRange` 2 6)))

(event `UpdateSMRotation`
  ; If the slider value changes, update the rotation of the tooth
  (if (`self.IsThisExtractableSelected`)
    (`SceneComponent.K2_SetRelativeRotation` (`self.Ref_SM`) (`KismetMathLibrary.MakeRotator` (+ (* (* (- (`self.Rotation01`) 0.5) 2.0) (`self.MaxAngle`)) 90.0)) false false)))

(event `self.BoxCollision.OnComponentBeginOverlap`
  (params (OverlappedComponent :type "PrimitiveComponent Object Reference") (OtherActor :type "Actor Object Reference") (OtherComp :type "PrimitiveComponent Object Reference") (OtherBodyIndex :type Integer) (bFromSweep :type Boolean) (SweepResult :type "HitResult Structure (by ref)"))
  ; Collision extraction done
  (if (== OtherComp (`self.StaticMesh`))
    (`ActorComponent.K2_DestroyComponent` (`self.StaticMesh`))
    (set `self.ExtractionDone` true)))

(fn `UserConstructionScript`)